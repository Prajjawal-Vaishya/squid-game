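; Red Light, Green Light doll actor, as in Squid Game, that turns its head between the two phases.
; Tick runs a one-time intro sound and delay, then shows a Timer widget and enables player walking.
; After the intro it calls the character's KillPlayer every tick.
; A random Delay on Tick drives a FlipFlop that plays voice cues and rotation timelines, toggling the RedLight flag.
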(event `self.ReceiveBeginPlay`
  (bind _asbp_third_person_character (cast `/Game/ThirdPerson/Blueprints/BP_ThirdPersonCharacter` (`GameplayStatics.GetPlayerCharacter` 0)))
  (set `self.CharacterRef` _asbp_third_person_character))

(event `self.ReceiveTick`
  (params (DeltaSeconds :type "Float (single-precision)"))
  (if (`self.bGameStarting`)
    (`/Engine/EditorBlueprintResources/StandardMacros.DoOnce` false
      (:`Completed`
        (`GameplayStatics.PlaySoundAtLocation` "/Game/LevelPrototyping/Sounds/SoundEffects/Voicy_SQUID_GAME_ROUND_SOUND_EFFECT___NO_COPYRIGHT.Voicy_SQUID_GAME_ROUND_SOUND_EFFECT___NO_COPYRIGHT" (0.0 0.0 0.0) (struct) 1.0 1.0 0.0 null null null null)
        (`KismetSystemLibrary.Delay` 12.0)
        (bind _returnvalue (`|CreateWidget` "/Game/Blueprints/Timer.Timer_C"))
        (`UserWidget.AddToViewport` _returnvalue 0)
        (set `self.bGameStarting` false)
        (`CharacterMovementComponent.SetMovementMode` (`Character.CharacterMovement` (`self.CharacterRef`)) "MOVE_Walking" 0)))
    (else
      (`/Game/ThirdPerson/Blueprints/BP_ThirdPersonCharacter.KillPlayer` (`self.CharacterRef`))))
  (`KismetSystemLibrary.Delay` (`KismetMathLibrary.RandomFloatInRange` 2.0 6.0))
  (`self.Move Doll Head`))

(event `Move Doll Head`
  (`/Engine/EditorBlueprintResources/StandardMacros.FlipFlop`
    (:`A`
      (`GameplayStatics.PlaySoundAtLocation` "/Game/LevelPrototyping/Sounds/SoundEffects/Voicy_Red_Light.Voicy_Red_Light" (0.0 0.0 0.0) (struct) 1.0 1.0 0.0 null null null null)
      (`KismetSystemLibrary.Delay` 0.2)
      (bind (_direction _rotation) (`Timeline|RedLightRotationSpeed` :!via `PlayFromStart`)
        (:`Update`
          (`SceneComponent.K2_SetRelativeRotation` (`self.StaticMesh1`) (`KismetMathLibrary.MakeRotator` 0.0 0.0 _rotation) false false))
        (:`Finished`
          (set `self.bRedLight` true))))
    (:`B`
      (set `self.bRedLight` false)
      (`GameplayStatics.PlaySoundAtLocation` "/Game/LevelPrototyping/Sounds/SoundEffects/Voicy_Green_Light.Voicy_Green_Light" (0.0 0.0 0.0) (struct) 1.0 1.0 0.0 null null null null)
      (bind (_direction_2 _rotation_2) (`Timeline|GreenLightRotationSpeed` :!via `PlayFromStart`)
        (:`Update`
          (`SceneComponent.K2_SetRelativeRotation` (`self.StaticMesh1`) (`KismetMathLibrary.MakeRotator` 0.0 0.0 _rotation_2) false false))))))

(fn `UserConstructionScript`)
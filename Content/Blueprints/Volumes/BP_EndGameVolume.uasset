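; End-game trigger volume that completes the game when the player character enters it.
; BeginPlay caches the player's BP_ThirdPersonCharacter.
; Begin overlap compares the overlapping component, not the actor, to that reference, then prints a debug string, sets InWinnerZone and calls CompleteGame on the character.
; End overlap compares the actor and clears InWinnerZone.
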(event `self.ReceiveBeginPlay`
  (bind _asbp_third_person_character (cast `/Game/ThirdPerson/Blueprints/BP_ThirdPersonCharacter` (`GameplayStatics.GetPlayerCharacter` 0)))
  (set `self.CharacterRef` _asbp_third_person_character))

(event `self.EndGameCollision.OnComponentBeginOverlap`
  (params (OverlappedComponent :type "PrimitiveComponent Object Reference") (OtherActor :type "Actor Object Reference") (OtherComp :type "PrimitiveComponent Object Reference") (OtherBodyIndex :type Integer) (bFromSweep :type Boolean) (SweepResult :type "HitResult Structure (by ref)"))
  (bind _characterref (`self.CharacterRef`))
  (if (== OtherComp (`self.CharacterRef`))
    (`KismetSystemLibrary.PrintString` "Hello")
    (set `/Game/ThirdPerson/Blueprints/BP_ThirdPersonCharacter.bInWinnerZone` true _characterref)
    (`/Game/ThirdPerson/Blueprints/BP_ThirdPersonCharacter.Complete Game` _characterref)))

(event `self.EndGameCollision.OnComponentEndOverlap`
  (params (OverlappedComponent :type "PrimitiveComponent Object Reference") (OtherActor :type "Actor Object Reference") (OtherComp :type "PrimitiveComponent Object Reference") (OtherBodyIndex :type Integer))
  (if (== OtherActor (`self.CharacterRef`))
    (set `/Game/ThirdPerson/Blueprints/BP_ThirdPersonCharacter.bInWinnerZone` false (`self.CharacterRef`))))

(fn `UserConstructionScript`)